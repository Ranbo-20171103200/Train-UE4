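; BP_Statue is a statue actor that can be switched on and off to show a rotating text, spotlight, sparks and audio.
; It starts inactive, hiding the text and light and deactivating the sparks and audio on BeginPlay.
; SetStatueActive toggles all four components and a RotatingText flag.
; While that flag is set, Tick spins the text in yaw at a frame-rate-independent speed.
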(event `self.ReceiveBeginPlay`
  (`SceneComponent.SetVisibility` (`self.TextRender`) false false)
  (`SceneComponent.SetVisibility` (`self.SpotLight`) false false)
  (`ActorComponent.SetActive` (`self.Sparks`) false false)
  (`ActorComponent.SetActive` (`self.Audio`) false false))

(event `self.ReceiveTick`
  (params (DeltaSeconds :type "Float (single-precision)"))
  (if (`self.RotatingText`)
    (`SceneComponent.K2_AddLocalRotation` (`self.TextRender`) (`KismetMathLibrary.MakeRotator` 0.0 0.0 (* DeltaSeconds 180.0)) false false)))

(fn `SetStatueActive`
  (params (Active :type Boolean))
  (if Active
    (set `self.RotatingText` true)
    (`SceneComponent.SetVisibility` (`self.TextRender`) true false)
    (`SceneComponent.SetVisibility` (`self.SpotLight`) true false)
    (`ActorComponent.SetActive` (`self.Sparks`) true false)
    (`ActorComponent.SetActive` (`self.Audio`) true false)
    (else
      (set `self.RotatingText` false)
      (`SceneComponent.SetVisibility` (`self.TextRender`) false false)
      (`SceneComponent.SetVisibility` (`self.SpotLight`) false false)
      (`ActorComponent.SetActive` (`self.Sparks`) false false)
      (`ActorComponent.SetActive` (`self.Audio`) false false))))

(fn `UserConstructionScript`)